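; BP_CoopGameState is the game state for a co-op prototype, acting as a shared registry of gameplay objects.
; Separate functions register grabbables, players, bombs, breakables and plates, each adding its argument uniquely to a matching array.
; It only stores these lists, with no removal functions and no active event or construction logic.
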(event EventBeginPlay)

(event EventTick
  (params (DeltaSeconds :type Float%20%28single-precision%29)))

(fn ConstructionScript)

(fn RegGrabbable
  (params (A :type Actor%20Object%20Reference))
  (Utilities|Array|AddUnique (Variables|Default|GetRegGrabbables) A))

(fn RegPlayer
  (params (A :type Actor%20Object%20Reference))
  (Utilities|Array|AddUnique (Variables|Default|GetRegPlayers) A))

(fn RegBomb
  (params (A :type Actor%20Object%20Reference))
  (Utilities|Array|AddUnique (Variables|Default|GetRegBombs) A))

(fn RegBreakable
  (params (A :type Actor%20Object%20Reference))
  (Utilities|Array|AddUnique (Variables|Default|GetRegBreakables) A))

(fn RegPlate
  (params (A :type Actor%20Object%20Reference))
  (Utilities|Array|AddUnique (Variables|Default|GetRegPlates) A))