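; Honey puddle hazard that slows blob characters within its radius and can stick grabbable props lying close to its surface plane.
; Each Tick it polls actors by class and distance, refreshing a short slow timer on blobs and calling StickHere on props when StickProps is on.
; A Niagara effect draws it oriented to the surface.
; With a positive lifetime it shrinks away, then unsticks props in range and destroys itself.
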(event EventBeginPlay
  (Niagara|SetNiagaraVariable(Float) (Variables|Default|GetNiagara) "User.PuddleSize" (* (Variables|Default|GetRadius) (Math|Float|MakeLiteralFloat 2.2)))
  (Niagara|SetNiagaraVariable(Float) (Variables|Default|GetNiagara) "User.Shrink01" 1.0)
  (Niagara|SetNiagaraVariable(Vector3) (Variables|Default|GetNiagara) "User.SurfaceNormal" (Transformation|GetActorUpVector))
  (Niagara|SetNiagaraVariable(Vector3) (Variables|Default|GetNiagara) "User.SurfaceTangent" (Transformation|GetActorForwardVector)))

(event Collision|EventActorBeginOverlap
  (params (OtherActor :type Actor%20Object%20Reference)))

(event EventTick
  (params (DeltaSeconds :type Float%20%28single-precision%29))
  (bind _returnvalue (Transformation|GetActorLocation))
  (bind _outactors (Actor|GetAllActorsOfClass "/Game/Proto/Blueprints/BP_BlobCharacter.BP_BlobCharacter_C"))
  (for _array_element _outactors
    (if (< (Math|Vector|VectorLength (- (Transformation|GetActorLocation _array_element) _returnvalue)) (Variables|Default|GetRadius))
      (Variables|/Game/Proto/Blueprints/BP_BlobCharacter.BP_BlobCharacter_C|SetEnvSlow _array_element (Variables|Default|GetSlowFactor))
      (Variables|/Game/Proto/Blueprints/BP_BlobCharacter.BP_BlobCharacter_C|SetEnvSlowTimer _array_element 0.2)))
  (if (Variables|Default|GetStickProps)
    (bind _outactors_2 (Actor|GetAllActorsOfClass "/Game/Proto/Blueprints/BP_Grabbable.BP_Grabbable_C"))
    (for _array_element_2 _outactors_2
      (if (and (< (Math|Vector|VectorLength (- (Transformation|GetActorLocation _array_element_2) _returnvalue)) (Variables|Default|GetRadius)) (< (Math|Float|Absolute(Float) (Math|Vector|DotProduct (- (Transformation|GetActorLocation _array_element_2) _returnvalue) (Transformation|GetActorUpVector))) (Math|Float|MakeLiteralFloat 7e+01)))
        (Default|StickHere _array_element_2))))
  (if (> (Variables|Default|GetLifeSeconds) (Math|Float|MakeLiteralFloat 0.0))
    (Variables|Default|SetAgeTimer (+ (Variables|Default|GetAgeTimer) DeltaSeconds))
    (Niagara|SetNiagaraVariable(Float) (Variables|Default|GetNiagara) "User.Shrink01" (Math|Float|Clamp(Float) (Math|Float|SafeDivide (- (Variables|Default|GetLifeSeconds) (Variables|Default|GetAgeTimer)) (select (> (Variables|Default|GetShrinkTime) (Math|Float|MakeLiteralFloat 0.05)) (Variables|Default|GetShrinkTime) (Math|Float|MakeLiteralFloat 1.2)))))
    (if (> (Variables|Default|GetAgeTimer) (+ (Variables|Default|GetLifeSeconds) (Math|Float|MakeLiteralFloat 0.15)))
      (bind _outactors_3 (Actor|GetAllActorsOfClass "/Game/Proto/Blueprints/BP_Grabbable.BP_Grabbable_C"))
      (for _array_element_3 _outactors_3
        (if (< (Math|Vector|VectorLength (- (Transformation|GetActorLocation _array_element_3) _returnvalue)) (Variables|Default|GetRadius))
          (Default|Unstick _array_element_3)))
      (Actor|DestroyActor self))))

(fn ConstructionScript
  (Niagara|SetNiagaraVariable(Float) (Variables|Default|GetNiagara) "User.PuddleSize" (* (Variables|Default|GetRadius) (Math|Float|MakeLiteralFloat 2.2)))
  (Niagara|SetNiagaraVariable(Vector3) (Variables|Default|GetNiagara) "User.SurfaceNormal" (Transformation|GetActorUpVector))
  (Niagara|SetNiagaraVariable(Vector3) (Variables|Default|GetNiagara) "User.SurfaceTangent" (Transformation|GetActorForwardVector)))