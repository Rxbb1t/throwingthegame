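; Hex-grid floor whose tiles rise, grow and fade in near BP_BlobCharacter actors (two tracked) and sink away elsewhere.
; Construction script builds a hexagon of tile, outline and collision instances; the collision instances never move, so the whole field stays solid.
; Tick eases each tile's height by distance to the nearer character, and ApplyTile writes transforms and fade custom data.
; Render state is dirtied once per changed frame to batch instance updates.
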(event EventBeginPlay
  (Variables|Default|SetIdx 0)
  (for _array_element (Variables|Default|GetTilePos)
    (Utilities|Array|SetArrayElem (Variables|Default|GetTileZ) (Variables|Default|GetIdx) (- (Math|Float|MakeLiteralFloat 0.0) (Variables|Default|GetRiseDepth)))
    (CallFunction|ApplyTile (Variables|Default|GetIdx) _array_element (- (Math|Float|MakeLiteralFloat 0.0) (Variables|Default|GetRiseDepth)) 0.0 false)
    (Variables|Default|SetIdx (+ (Variables|Default|GetIdx) (Class|KismetSystemLibrary|MakeLiteralInteger 1))))
  (CallFunction|ApplyTile 0 (Utilities|Array|Get(acopy) (Variables|Default|GetTilePos)) (- (Math|Float|MakeLiteralFloat 0.0) (Variables|Default|GetRiseDepth)) 0.0 true))

(event EventTick
  (params (DeltaSeconds :type Float%20%28single-precision%29))
  (Variables|Default|SetbHasB false)
  (Variables|Default|SetIdx 0)
  (bind _outactors (Actor|GetAllActorsOfClass "/Game/Proto/Blueprints/BP_BlobCharacter.BP_BlobCharacter_C"))
  (for _array_element _outactors
    (if (== (Variables|Default|GetIdx) (Class|KismetSystemLibrary|MakeLiteralInteger))
      (Variables|Default|SetPlayerA (- (Transformation|GetActorLocation _array_element) (Transformation|GetActorLocation)))
      (else
        (Variables|Default|SetPlayerB (- (Transformation|GetActorLocation _array_element) (Transformation|GetActorLocation)))
        (Variables|Default|SetbHasB true)))
    (Variables|Default|SetIdx (+ (Variables|Default|GetIdx) (Class|KismetSystemLibrary|MakeLiteralInteger 1))))
  (Variables|Default|SetIdx 0)
  (Variables|Default|SetTouched 0)
  (for _array_element_2 (Variables|Default|GetTilePos)
    (Variables|Default|SetTmpNear (Math|Float|Sqrt (+ (* (- (.X (Math|Vector|BreakVector _array_element_2)) (.X (Math|Vector|BreakVector (Variables|Default|GetPlayerA)))) (- (.X (Math|Vector|BreakVector _array_element_2)) (.X (Math|Vector|BreakVector (Variables|Default|GetPlayerA))))) (* (- (.Y (Math|Vector|BreakVector _array_element_2)) (.Y (Math|Vector|BreakVector (Variables|Default|GetPlayerA)))) (- (.Y (Math|Vector|BreakVector _array_element_2)) (.Y (Math|Vector|BreakVector (Variables|Default|GetPlayerA))))))))
    (if (Variables|Default|GetbHasB)
      (Variables|Default|SetTmpB (Math|Float|Sqrt (+ (* (- (.X (Math|Vector|BreakVector _array_element_2)) (.X (Math|Vector|BreakVector (Variables|Default|GetPlayerB)))) (- (.X (Math|Vector|BreakVector _array_element_2)) (.X (Math|Vector|BreakVector (Variables|Default|GetPlayerB))))) (* (- (.Y (Math|Vector|BreakVector _array_element_2)) (.Y (Math|Vector|BreakVector (Variables|Default|GetPlayerB)))) (- (.Y (Math|Vector|BreakVector _array_element_2)) (.Y (Math|Vector|BreakVector (Variables|Default|GetPlayerB))))))))
      (Variables|Default|SetTmpNear (select (< (Variables|Default|GetTmpB) (Variables|Default|GetTmpNear)) (Variables|Default|GetTmpB) (Variables|Default|GetTmpNear))))
    (Variables|Default|SetTmpTarget (select (< (Variables|Default|GetTmpNear) (Variables|Default|GetRevealRadius)) (Math|Float|MakeLiteralFloat 0.0) (- (Math|Float|MakeLiteralFloat 0.0) (Variables|Default|GetRiseDepth))))
    (Variables|Default|SetTmpCur (Utilities|Array|Get(acopy) (Variables|Default|GetTileZ) (Variables|Default|GetIdx)))
    (if (> (Math|Float|Absolute(Float) (- (Variables|Default|GetTmpTarget) (Variables|Default|GetTmpCur))) (Math|Float|MakeLiteralFloat 0.5))
      (Variables|Default|SetTmpZ (Math|Interpolation|FInterpTo (Variables|Default|GetTmpCur) (Variables|Default|GetTmpTarget) DeltaSeconds (Variables|Default|GetRiseSpeed)))
      (Utilities|Array|SetArrayElem (Variables|Default|GetTileZ) (Variables|Default|GetIdx) (Variables|Default|GetTmpZ))
      (CallFunction|ApplyTile (Variables|Default|GetIdx) _array_element_2 (Variables|Default|GetTmpZ) (Math|Float|Clamp(Float) (Math|Float|SafeDivide (+ (Variables|Default|GetTmpZ) (Variables|Default|GetRiseDepth)) (Variables|Default|GetFadeSpan))) false)
      (Variables|Default|SetTouched (+ (Variables|Default|GetTouched) (Class|KismetSystemLibrary|MakeLiteralInteger 1))))
    (Variables|Default|SetIdx (+ (Variables|Default|GetIdx) (Class|KismetSystemLibrary|MakeLiteralInteger 1))))
  (if (> (Variables|Default|GetTouched) (Class|KismetSystemLibrary|MakeLiteralInteger))
    (CallFunction|ApplyTile 0 (Utilities|Array|Get(acopy) (Variables|Default|GetTilePos)) (Utilities|Array|Get(acopy) (Variables|Default|GetTileZ)) (Math|Float|Clamp(Float) (Math|Float|SafeDivide (+ (Utilities|Array|Get(acopy) (Variables|Default|GetTileZ)) (Variables|Default|GetRiseDepth)) (Variables|Default|GetFadeSpan))) true)))

(fn ConstructionScript
  (bind _hexradius (Variables|Default|GetHexRadius))
  (bind _outlinewidth (Variables|Default|GetOutlineWidth))
  (bind _hexradius_2 (Variables|Default|GetHexRadius))
  (bind _returnvalue (- _hexradius _outlinewidth))
  (bind _returnvalue_2 (Math|Float|SafeDivide _returnvalue _hexradius_2))
  (Collision|SetCollisionEnabled (Variables|Default|GetTiles) "NoCollision")
  (Collision|SetCollisionEnabled (Variables|Default|GetOutlines) "NoCollision")
  (Collision|SetCollisionEnabled (Variables|Default|GetCollide) "QueryAndPhysics")
  (Components|InstancedStaticMesh|ClearInstances (Variables|Default|GetTiles))
  (Components|InstancedStaticMesh|ClearInstances (Variables|Default|GetOutlines))
  (Components|InstancedStaticMesh|ClearInstances (Variables|Default|GetCollide))
  (Utilities|Array|Clear (Variables|Default|GetTilePos))
  (Utilities|Array|Clear (Variables|Default|GetTileZ))
  (Variables|Default|SetRevealRadius (* (Variables|Default|GetRevealTiles) (* (Math|Float|MakeLiteralFloat 1.7320508) (Variables|Default|GetHexRadius))))
  (Variables|Default|SetSide (+ (* (Class|KismetSystemLibrary|MakeLiteralInteger 2) (Variables|Default|GetFieldRings)) (Class|KismetSystemLibrary|MakeLiteralInteger 1)))
  (Utilities|Array|Resize (Variables|Default|GetScratch) (* (Variables|Default|GetSide) (Variables|Default|GetSide)))
  (Variables|Default|SetInstIdx 0)
  (Variables|Default|SetTmpQ (- (Class|KismetSystemLibrary|MakeLiteralInteger) (Variables|Default|GetFieldRings)))
  (Variables|Default|SetTmpR (- (- (Class|KismetSystemLibrary|MakeLiteralInteger) (Variables|Default|GetFieldRings)) (Class|KismetSystemLibrary|MakeLiteralInteger 1)))
  (for _array_element (Variables|Default|GetScratch)
    (Variables|Default|SetTmpR (+ (Variables|Default|GetTmpR) (Class|KismetSystemLibrary|MakeLiteralInteger 1)))
    (if (> (Variables|Default|GetTmpR) (Variables|Default|GetFieldRings))
      (Variables|Default|SetTmpR (- (Class|KismetSystemLibrary|MakeLiteralInteger) (Variables|Default|GetFieldRings)))
      (Variables|Default|SetTmpQ (+ (Variables|Default|GetTmpQ) (Class|KismetSystemLibrary|MakeLiteralInteger 1))))
    (if (not (> (Math|Float|Absolute(Float) (Math|Conversions|ToFloat(Integer) (+ (Variables|Default|GetTmpQ) (Variables|Default|GetTmpR)))) (Math|Conversions|ToFloat(Integer) (Variables|Default|GetFieldRings))))
      (Variables|Default|SetTmpX (* (* (Math|Float|MakeLiteralFloat 1.5) (Variables|Default|GetHexRadius)) (Math|Conversions|ToFloat(Integer) (Variables|Default|GetTmpQ))))
      (Variables|Default|SetTmpY (* (* (Math|Float|MakeLiteralFloat 1.7320508) (Variables|Default|GetHexRadius)) (+ (Math|Conversions|ToFloat(Integer) (Variables|Default|GetTmpR)) (* (Math|Float|MakeLiteralFloat 0.5) (Math|Conversions|ToFloat(Integer) (Variables|Default|GetTmpQ))))))
      (Utilities|Array|Add (Variables|Default|GetTilePos) (Math|Vector|MakeVector (Variables|Default|GetTmpX) (Variables|Default|GetTmpY) 0.0))
      (Utilities|Array|Add (Variables|Default|GetTileZ) 0.0)
      (Components|InstancedStaticMesh|AddInstance (Variables|Default|GetOutlines) (Math|Transform|MakeTransform (Math|Vector|MakeVector (Variables|Default|GetTmpX) (Variables|Default|GetTmpY) 0.0) (Math|Rotator|MakeRotator 0.0 0.0 0.0) (Math|Vector|MakeVector 1.0 1.0 (Variables|Default|GetTileThick))) false)
      (Components|InstancedStaticMesh|AddInstance (Variables|Default|GetTiles) (Math|Transform|MakeTransform (Math|Vector|MakeVector (Variables|Default|GetTmpX) (Variables|Default|GetTmpY) (Variables|Default|GetTileLift)) (Math|Rotator|MakeRotator 0.0 0.0 0.0) (Math|Vector|MakeVector _returnvalue_2 _returnvalue_2 (Variables|Default|GetTileThick))) false)
      (Components|InstancedStaticMesh|AddInstance (Variables|Default|GetCollide) (Math|Transform|MakeTransform (Math|Vector|MakeVector (Variables|Default|GetTmpX) (Variables|Default|GetTmpY) 0.0) (Math|Rotator|MakeRotator 0.0 0.0 0.0) (Math|Vector|MakeVector 1.0 1.0 (Variables|Default|GetTileThick))) false)
      (Components|InstancedStaticMesh|SetCustomDataValue (Variables|Default|GetTiles) (Variables|Default|GetInstIdx) 0 1.0 false)
      (Components|InstancedStaticMesh|SetCustomDataValue (Variables|Default|GetOutlines) (Variables|Default|GetInstIdx) 0 1.0 false)
      (Variables|Default|SetInstIdx (+ (Variables|Default|GetInstIdx) (Class|KismetSystemLibrary|MakeLiteralInteger 1))))))

(fn ApplyTile
  (params (Index :type Integer) (Pos :type Vector) (Z :type Float%20%28double-precision%29) (Fade :type Float%20%28double-precision%29) (Dirty :type Boolean))
  (bind _hexradius (Variables|Default|GetHexRadius))
  (bind _outlinewidth (Variables|Default|GetOutlineWidth))
  (bind _hexradius_2 (Variables|Default|GetHexRadius))
  (bind _mintilescale (Variables|Default|GetMinTileScale))
  (bind _returnvalue (Math|Float|Lerp _mintilescale 1.0 Fade))
  (bind _returnvalue_2 (- _hexradius _outlinewidth))
  (bind _returnvalue_3 (Math|Float|SafeDivide _returnvalue_2 _hexradius_2))
  (Components|InstancedStaticMesh|UpdateInstanceTransform (Variables|Default|GetOutlines) Index (Math|Transform|MakeTransform (+ Pos (Math|Vector|MakeVector 0.0 0.0 Z)) (Math|Rotator|MakeRotator 0.0 0.0 0.0) (Math|Vector|MakeVector _returnvalue _returnvalue (Variables|Default|GetTileThick))) false Dirty false)
  (Components|InstancedStaticMesh|UpdateInstanceTransform (Variables|Default|GetTiles) Index (Math|Transform|MakeTransform (+ Pos (Math|Vector|MakeVector 0.0 0.0 (+ Z (Variables|Default|GetTileLift)))) (Math|Rotator|MakeRotator 0.0 0.0 0.0) (Math|Vector|MakeVector (* _returnvalue_3 _returnvalue) (* _returnvalue_3 _returnvalue) (Variables|Default|GetTileThick))) false Dirty false)
  (Components|InstancedStaticMesh|SetCustomDataValue (Variables|Default|GetTiles) Index 0 Fade Dirty)
  (Components|InstancedStaticMesh|SetCustomDataValue (Variables|Default|GetOutlines) Index 0 Fade Dirty))