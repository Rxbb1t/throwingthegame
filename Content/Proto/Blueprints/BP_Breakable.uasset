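; Breakable block prop that shatters into flying debris with a click sound and can respawn after a delay.
; Shatter hides Body, disables its collision and spawns instanced-mesh chunks with outward velocity and random spin.
; Tick animates them through hand-integrated gravity and rotation rather than physics, clearing them after their lifetime.
; Tick also retries registering the actor with BP_CoopGameState until it succeeds; Shatter has no caller here.
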(event EventBeginPlay
  (Variables|Default|SetbBroken false)
  (Variables|Default|SetChunkT 99.0)
  (Variables|Default|SetRespawnTimer 0.0)
  (if (< (Variables|Default|GetBlockScale) (Math|Float|MakeLiteralFloat 0.01))
    (Variables|Default|SetBlockScale 1.0))
  (if (< (Variables|Default|GetChunkCount) (Class|KismetSystemLibrary|MakeLiteralInteger 1))
    (Variables|Default|SetChunkCount 30))
  (if (< (Variables|Default|GetChunkLife) (Math|Float|MakeLiteralFloat 0.01))
    (Variables|Default|SetChunkLife 1.6))
  (if (< (Variables|Default|GetChunkSpeed) (Math|Float|MakeLiteralFloat 1.0))
    (Variables|Default|SetChunkSpeed 3.4e+02))
  (if (< (Variables|Default|GetChunkUp) (Math|Float|MakeLiteralFloat 1.0))
    (Variables|Default|SetChunkUp 3.2e+02))
  (if (< (Variables|Default|GetChunkSize) (Math|Float|MakeLiteralFloat 0.001))
    (Variables|Default|SetChunkSize 0.16))
  (if (> (Variables|Default|GetChunkGravity) (Math|Float|MakeLiteralFloat -1.0))
    (Variables|Default|SetChunkGravity -1.4e+03))
  (if (< (Variables|Default|GetRespawnDelay) (Math|Float|MakeLiteralFloat 0.01))
    (Variables|Default|SetRespawnDelay 6.0))
  (Components|InstancedStaticMesh|ClearInstances (Variables|Default|GetChunks)))

(event EventTick
  (params (DeltaSeconds :type Float%20%28single-precision%29))
  (CallFunction|EnsureRegBreak)
  (if (Variables|Default|GetbBroken)
    (CallFunction|UpdateChunks DeltaSeconds)
    (Variables|Default|SetRespawnTimer (- (Variables|Default|GetRespawnTimer) DeltaSeconds))
    (if (Variables|Default|GetbRespawns)
      (if (< (Variables|Default|GetRespawnTimer) (Math|Float|MakeLiteralFloat 0.0))
        (CallFunction|Restore)))))

(fn ConstructionScript
  (bind _body (Variables|Default|GetBody))
  (bind _chunks (Variables|Default|GetChunks))
  (bind _blockscale (Variables|Default|GetBlockScale))
  (Transformation|SetRelativeScale3D _body (Math|Vector|MakeVector _blockscale _blockscale _blockscale))
  (Rendering|Material|SetMaterial _body 0 "/Game/Proto/Materials/MI_Breakable.MI_Breakable")
  (Rendering|Material|SetMaterial _chunks 0 "/Game/Proto/Materials/MI_Breakable.MI_Breakable")
  (Collision|SetCollisionEnabled _chunks "NoCollision")
  (Components|StaticMesh|SetStaticMesh (Variables|Default|GetChunkA) "/Engine/BasicShapes/Cube.Cube")
  (Transformation|SetRelativeScale3D (Variables|Default|GetChunkA) (Math|Vector|MakeVector 0.78 0.78 0.78))
  (Transformation|SetRelativeLocation (Variables|Default|GetChunkA) (Math|Vector|MakeVector 0.0 0.0 0.0) false false)
  (Transformation|SetRelativeRotation (Variables|Default|GetChunkA) (Math|Rotator|MakeRotator 0.0 12.0 35.0) false false)
  (Rendering|Material|SetMaterial (Variables|Default|GetChunkA) 0 "/Game/Proto/Materials/MI_BreakTrim.MI_BreakTrim")
  (Collision|SetCollisionEnabled (Variables|Default|GetChunkA) "NoCollision")
  (Components|StaticMesh|SetStaticMesh (Variables|Default|GetChunkB) "/Engine/BasicShapes/Cube.Cube")
  (Transformation|SetRelativeScale3D (Variables|Default|GetChunkB) (Math|Vector|MakeVector 0.5 0.5 0.5))
  (Transformation|SetRelativeLocation (Variables|Default|GetChunkB) (Math|Vector|MakeVector 12.0 -9.0 3e+01) false false)
  (Transformation|SetRelativeRotation (Variables|Default|GetChunkB) (Math|Rotator|MakeRotator 22.0 0.0 -25.0) false false)
  (Rendering|Material|SetMaterial (Variables|Default|GetChunkB) 0 "/Game/Proto/Materials/MI_BreakTrim.MI_BreakTrim")
  (Collision|SetCollisionEnabled (Variables|Default|GetChunkB) "NoCollision"))

(fn Shatter
  (bind _returnvalue (Transformation|GetActorLocation))
  (bind _returnvalue_2 (Math|Float|MakeLiteralFloat 5e+01))
  (bind _body (Variables|Default|GetBody))
  (bind _chunks (Variables|Default|GetChunks))
  (bind _blockscale (Variables|Default|GetBlockScale))
  (bind _chunksize (Variables|Default|GetChunkSize))
  (bind _returnvalue_3 (* _returnvalue_2 _blockscale))
  (if (not (Variables|Default|GetbBroken))
    (Variables|Default|SetbBroken true)
    (Variables|Default|SetRespawnTimer (Variables|Default|GetRespawnDelay))
    (Rendering|SetVisibility _body false true)
    (Collision|SetCollisionEnabled _body "NoCollision")
    (Audio|PlaySoundatLocation "/Engine/VREditor/Sounds/VR_click2_Cue.VR_click2_Cue" _returnvalue "0, 0, 0" 0.8 0.5 0.0 0 0 0 0)
    (Components|InstancedStaticMesh|ClearInstances _chunks)
    (Utilities|Array|Resize (Variables|Default|GetChunkPos) (Variables|Default|GetChunkCount))
    (Utilities|Array|Resize (Variables|Default|GetChunkVel) (Variables|Default|GetChunkCount))
    (Utilities|Array|Resize (Variables|Default|GetChunkRot) (Variables|Default|GetChunkCount))
    (Utilities|Array|Resize (Variables|Default|GetChunkSpin) (Variables|Default|GetChunkCount))
    (Variables|Default|SetChunkIdx 0)
    (for _array_element (Variables|Default|GetChunkPos)
      (Utilities|Array|SetArrayElem (Variables|Default|GetChunkPos) (Variables|Default|GetChunkIdx) (+ _returnvalue (* (Math|Random|RandomUnitVector) (* _returnvalue_3 (Math|Random|RandomFloatinRange 0.25 1.0)))))
      (Utilities|Array|SetArrayElem (Variables|Default|GetChunkVel) (Variables|Default|GetChunkIdx) (+ (* (- (Utilities|Array|Get(acopy) (Variables|Default|GetChunkPos) (Variables|Default|GetChunkIdx)) _returnvalue) (Math|Float|SafeDivide (Variables|Default|GetChunkSpeed) _returnvalue_3)) (Math|Vector|MakeVector 0.0 0.0 (Variables|Default|GetChunkUp))))
      (Utilities|Array|SetArrayElem (Variables|Default|GetChunkRot) (Variables|Default|GetChunkIdx) (Math|Vector|MakeVector 0.0 0.0 0.0))
      (Utilities|Array|SetArrayElem (Variables|Default|GetChunkSpin) (Variables|Default|GetChunkIdx) (* (Math|Random|RandomUnitVector) (Math|Float|MakeLiteralFloat 6.2e+02)))
      (Components|InstancedStaticMesh|AddInstance _chunks (Math|Transform|MakeTransform (Utilities|Array|Get(acopy) (Variables|Default|GetChunkPos) (Variables|Default|GetChunkIdx)) (Math|Rotator|MakeRotator 0.0 0.0 0.0) (Math|Vector|MakeVector _chunksize _chunksize _chunksize)) true)
      (Variables|Default|SetChunkIdx (+ (Variables|Default|GetChunkIdx) (Class|KismetSystemLibrary|MakeLiteralInteger 1))))
    (Variables|Default|SetChunkT 0.0)))

(fn UpdateChunks
  (params (DeltaSec :type Float%20%28double-precision%29))
  (bind _chunks (Variables|Default|GetChunks))
  (bind _chunksize (Variables|Default|GetChunkSize))
  (if (< (Variables|Default|GetChunkT) (Variables|Default|GetChunkLife))
    (Variables|Default|SetChunkT (+ (Variables|Default|GetChunkT) DeltaSec))
    (Variables|Default|SetChunkIdx 0)
    (for _array_element (Variables|Default|GetChunkPos)
      (Utilities|Array|SetArrayElem (Variables|Default|GetChunkVel) (Variables|Default|GetChunkIdx) (+ (Utilities|Array|Get(acopy) (Variables|Default|GetChunkVel) (Variables|Default|GetChunkIdx)) (Math|Vector|MakeVector 0.0 0.0 (* (Variables|Default|GetChunkGravity) DeltaSec))))
      (Utilities|Array|SetArrayElem (Variables|Default|GetChunkPos) (Variables|Default|GetChunkIdx) (+ (Utilities|Array|Get(acopy) (Variables|Default|GetChunkPos) (Variables|Default|GetChunkIdx)) (* (Utilities|Array|Get(acopy) (Variables|Default|GetChunkVel) (Variables|Default|GetChunkIdx)) DeltaSec)))
      (Utilities|Array|SetArrayElem (Variables|Default|GetChunkRot) (Variables|Default|GetChunkIdx) (+ (Utilities|Array|Get(acopy) (Variables|Default|GetChunkRot) (Variables|Default|GetChunkIdx)) (* (Utilities|Array|Get(acopy) (Variables|Default|GetChunkSpin) (Variables|Default|GetChunkIdx)) DeltaSec)))
      (Components|InstancedStaticMesh|UpdateInstanceTransform _chunks (Variables|Default|GetChunkIdx) (Math|Transform|MakeTransform (Utilities|Array|Get(acopy) (Variables|Default|GetChunkPos) (Variables|Default|GetChunkIdx)) (Math|Rotator|MakeRotator (.X (Math|Vector|BreakVector (Utilities|Array|Get(acopy) (Variables|Default|GetChunkRot) (Variables|Default|GetChunkIdx)))) (.Y (Math|Vector|BreakVector (Utilities|Array|Get(acopy) (Variables|Default|GetChunkRot) (Variables|Default|GetChunkIdx)))) (.Z (Math|Vector|BreakVector (Utilities|Array|Get(acopy) (Variables|Default|GetChunkRot) (Variables|Default|GetChunkIdx))))) (Math|Vector|MakeVector _chunksize _chunksize _chunksize)) true true false)
      (Variables|Default|SetChunkIdx (+ (Variables|Default|GetChunkIdx) (Class|KismetSystemLibrary|MakeLiteralInteger 1))))
    (else
      (Components|InstancedStaticMesh|ClearInstances _chunks))))

(fn Restore
  (bind _body (Variables|Default|GetBody))
  (Variables|Default|SetbBroken false)
  (Variables|Default|SetChunkT 99.0)
  (Components|InstancedStaticMesh|ClearInstances (Variables|Default|GetChunks))
  (Rendering|SetVisibility _body true true)
  (Collision|SetCollisionEnabled _body "QueryAndPhysics"))

(fn EnsureRegBreak
  (if (not (Variables|Default|GetbRegistered))
    (bind _asbp_coop_game_state (Utilities|Casting|CastToBP_CoopGameState (Game|GetGameState)))
    (Variables|Default|SetGS _asbp_coop_game_state)
    (Default|RegBreakable _asbp_coop_game_state self)
    (Variables|Default|SetbRegistered true)))