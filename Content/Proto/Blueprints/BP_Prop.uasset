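; Generic prop actor that displays a configurable static mesh, with all its logic in the construction script.
; The script assigns PropMesh, then AlignToBase uses local bounds to offset it so the actor origin sits at the bottom center, or zeroes the offset when off.
; A NoCollision flag optionally disables the mesh's collision, and the event graph has no active logic.
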(event EventBeginPlay)

(event Collision|EventActorBeginOverlap
  (params (OtherActor :type Actor%20Object%20Reference)))

(event EventTick
  (params (DeltaSeconds :type Float%20%28single-precision%29)))

(fn ConstructionScript
  (bind _mesh (Variables|Default|GetMesh))
  (bind (_min _max) (Components|StaticMesh|GetLocalBounds _mesh))
  (Components|StaticMesh|SetStaticMesh _mesh (Variables|Default|GetPropMesh))
  (if (Variables|Default|GetAlignToBase)
    (Transformation|SetRelativeLocation _mesh (Math|Vector|MakeVector (- (Math|Float|MakeLiteralFloat 0.0) (/ (+ (.X (Math|Vector|BreakVector _min)) (.X (Math|Vector|BreakVector _max))) (Math|Float|MakeLiteralFloat 2.0))) (- (Math|Float|MakeLiteralFloat 0.0) (/ (+ (.Y (Math|Vector|BreakVector _min)) (.Y (Math|Vector|BreakVector _max))) (Math|Float|MakeLiteralFloat 2.0))) (- (Math|Float|MakeLiteralFloat 0.0) (.Z (Math|Vector|BreakVector _min)))) false false)
    (else
      (Transformation|SetRelativeLocation _mesh (Math|Vector|MakeVector 0.0 0.0 0.0) false false)))
  (if (Variables|Default|GetNoCollision)
    (Collision|SetCollisionEnabled _mesh "NoCollision")))