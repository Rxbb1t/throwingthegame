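; Gate actor whose door sinks when its linked pressure plates are active, requiring either all or any of them per RequireAll.
; On BeginPlay, a gate with no linked plates links itself to the nearest BP_PressurePlate.
; Tick polls plate states and eases OpenAmount with FInterpTo to slide the door vertically; an unconnected copy of this logic never runs.
; The construction script builds the door, posts, lintel and sill from scaled cubes.
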(event EventBeginPlay
  (if (== (Utilities|Array|Length (Variables|Default|GetLinkedPlates)) (Class|KismetSystemLibrary|MakeLiteralInteger))
    (Variables|Default|SetBestD 999999.0)
    (Variables|Default|SetbFoundPlate false)
    (bind _outactors (Actor|GetAllActorsOfClass "/Game/Proto/Blueprints/BP_PressurePlate.BP_PressurePlate_C"))
    (for _array_element _outactors
      (bind _asbp_pressure_plate (Utilities|Casting|CastToBP_PressurePlate _array_element))
      (Variables|Default|SetTmpD (Math|Vector|VectorLength (- (Transformation|GetActorLocation _array_element) (Transformation|GetActorLocation))))
      (if (< (Variables|Default|GetTmpD) (Variables|Default|GetBestD))
        (Variables|Default|SetBestD (Variables|Default|GetTmpD))
        (Variables|Default|SetNearestPlate _asbp_pressure_plate)
        (Variables|Default|SetbFoundPlate true)))
    (if (Variables|Default|GetbFoundPlate)
      (Utilities|Array|Add (Variables|Default|GetLinkedPlates) (Variables|Default|GetNearestPlate)))))

(event EventTick
  (params (DeltaSeconds :type Float%20%28single-precision%29))
  (bind _linkedplates (Variables|Default|GetLinkedPlates))
  (Variables|Default|SetbAllOn true)
  (Variables|Default|SetbAnyOn false)
  (for _array_element _linkedplates
    (if (Variables|/Game/Proto/Blueprints/BP_PressurePlate.BP_PressurePlate_C|GetbActive _array_element)
      (Variables|Default|SetbAnyOn true)
      (else
        (Variables|Default|SetbAllOn false))))
  (Variables|Default|SetbWantOpen (and (> (Utilities|Array|Length _linkedplates) (Class|KismetSystemLibrary|MakeLiteralInteger)) (select (Variables|Default|GetbRequireAll) (Variables|Default|GetbAllOn) (Variables|Default|GetbAnyOn))))
  (Variables|Default|SetOpenAmount (Math|Interpolation|FInterpTo (Variables|Default|GetOpenAmount) (select (Variables|Default|GetbWantOpen) (Math|Float|MakeLiteralFloat 1.0) (Math|Float|MakeLiteralFloat 0.0)) DeltaSeconds (Variables|Default|GetOpenSpeed)))
  (Transformation|SetRelativeLocation (Variables|Default|GetGateMesh) (Math|Vector|MakeVector 0.0 0.0 (- (Math|Float|MakeLiteralFloat 1.1e+02) (* (Variables|Default|GetOpenAmount) (Variables|Default|GetOpenHeight)))) false false))

(fn ConstructionScript
  (bind _gatemesh (Variables|Default|GetGateMesh))
  (Components|StaticMesh|SetStaticMesh _gatemesh "/Engine/BasicShapes/Cube.Cube")
  (Transformation|SetRelativeScale3D _gatemesh (Math|Vector|MakeVector 0.4 3.0 2.2))
  (Rendering|Material|SetMaterial _gatemesh 0 "/Game/Proto/Materials/MI_GateDoor.MI_GateDoor")
  (Components|StaticMesh|SetStaticMesh (Variables|Default|GetPostL) "/Engine/BasicShapes/Cube.Cube")
  (Transformation|SetRelativeScale3D (Variables|Default|GetPostL) (Math|Vector|MakeVector 0.72 0.58 2.62))
  (Transformation|SetRelativeLocation (Variables|Default|GetPostL) (Math|Vector|MakeVector 0.0 -179.0 131.0) false false)
  (Rendering|Material|SetMaterial (Variables|Default|GetPostL) 0 "/Game/Proto/Materials/MI_GateStone.MI_GateStone")
  (Collision|SetCollisionEnabled (Variables|Default|GetPostL) "QueryAndPhysics")
  (Components|StaticMesh|SetStaticMesh (Variables|Default|GetPostR) "/Engine/BasicShapes/Cube.Cube")
  (Transformation|SetRelativeScale3D (Variables|Default|GetPostR) (Math|Vector|MakeVector 0.72 0.58 2.62))
  (Transformation|SetRelativeLocation (Variables|Default|GetPostR) (Math|Vector|MakeVector 0.0 179.0 131.0) false false)
  (Rendering|Material|SetMaterial (Variables|Default|GetPostR) 0 "/Game/Proto/Materials/MI_GateStone.MI_GateStone")
  (Collision|SetCollisionEnabled (Variables|Default|GetPostR) "QueryAndPhysics")
  (Components|StaticMesh|SetStaticMesh (Variables|Default|GetLintel) "/Engine/BasicShapes/Cube.Cube")
  (Transformation|SetRelativeScale3D (Variables|Default|GetLintel) (Math|Vector|MakeVector 0.78 4.32 0.46))
  (Transformation|SetRelativeLocation (Variables|Default|GetLintel) (Math|Vector|MakeVector 0.0 0.0 285.0) false false)
  (Rendering|Material|SetMaterial (Variables|Default|GetLintel) 0 "/Game/Proto/Materials/MI_GateStone.MI_GateStone")
  (Collision|SetCollisionEnabled (Variables|Default|GetLintel) "QueryAndPhysics")
  (Components|StaticMesh|SetStaticMesh (Variables|Default|GetSill) "/Engine/BasicShapes/Cube.Cube")
  (Transformation|SetRelativeScale3D (Variables|Default|GetSill) (Math|Vector|MakeVector 0.86 4.32 0.14))
  (Transformation|SetRelativeLocation (Variables|Default|GetSill) (Math|Vector|MakeVector 0.0 0.0 7.0) false false)
  (Rendering|Material|SetMaterial (Variables|Default|GetSill) 0 "/Game/Proto/Materials/MI_GateStone.MI_GateStone")
  (Collision|SetCollisionEnabled (Variables|Default|GetSill) "QueryAndPhysics"))